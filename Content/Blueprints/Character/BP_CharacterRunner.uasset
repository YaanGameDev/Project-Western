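; BP_CharacterRunner is the runner character Blueprint, handling pause input and saving the coin high score on death.
; P branches on IsPauseMenuOpened to show or remove the pause widget, switching pause, cursor and input mode; this graph only ever clears that flag.
; DeathFunction calls its parent, pauses the game, then compares the game mode's TotalCoins against the HighScoreCoins save, creating or overwriting it as needed.
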(event EventDeathFunction
  ;[1 1 1] Save High Score for Coins
  (|CallParentFunction)
  (bind _asbp_main_game_mode_base (Utilities|Casting|CastToBP_MainGameModeBase (Game|GetGameMode)))
  (Game|SetGamePaused true)
  (bind _returnvalue (SaveGame|DoesSaveGameExist "HighscoreDataCoins"))
  (if _returnvalue
    (bind _returnvalue_2 (SaveGame|LoadGamefromSlot "HighscoreDataCoins"))
    (bind _output_get (Variables|Default|SetSaverSubClassCoins _returnvalue_2))
    (bind _ashigh_score_coins (Utilities|Casting|CastToHighScoreCoins _output_get))
    (if (> (Variables|/Script/ProjectWestern.MainGameModeBase|GetTotalCoins _asbp_main_game_mode_base) (Variables|/Game/Blueprints/HighScore/HighScoreCoins.HighScoreCoins_C|GetHighscore%20Value _ashigh_score_coins))
      (Variables|/Game/Blueprints/HighScore/HighScoreCoins.HighScoreCoins_C|SetHighscore%20Value _ashigh_score_coins (Variables|/Script/ProjectWestern.MainGameModeBase|GetTotalCoins _asbp_main_game_mode_base))
      (SaveGame|SaveGametoSlot (Variables|Default|GetSaverSubClassCoins) "HighscoreDataCoins"))
    (else
      (bind _returnvalue_3 (SaveGame|CreateSaveGameObject "/Game/Blueprints/HighScore/HighScoreCoins.HighScoreCoins_C"))
      (bind _output_get_2 (Variables|Default|SetSaverSubClassCoins _returnvalue_3))
      (bind _ashigh_score_coins_2 (Utilities|Casting|CastToHighScoreCoins _output_get_2))
      (Variables|/Game/Blueprints/HighScore/HighScoreCoins.HighScoreCoins_C|SetHighscore%20Value _ashigh_score_coins_2 (Variables|/Script/ProjectWestern.MainGameModeBase|GetTotalCoins _asbp_main_game_mode_base))
      (SaveGame|SaveGametoSlot (Variables|Default|GetSaverSubClassCoins) "HighscoreDataCoins"))))

(event Input|KeyboardEvents|P
  (params (Key :type Key%20Structure :default "None"))
  (bind _returnvalue (Game|GetPlayerController 0))
  ;[1 1 1] Pause Game System
  (:Pressed
    (if (not (Variables|Default|GetIsPauseMenuOpened%20?))
      (bind _returnvalue_2 (UserInterface|CreateWidget "/Game/HUD/PauseGame/HUD/HUD_PauseGame.HUD_PauseGame_C" _returnvalue))
      (bind _output_get (Variables|Default|SetPause%20Menu%20Widget _returnvalue_2))
      (UserInterface|Viewport|AddtoViewport _output_get 0)
      (Input|SetInputModeGameandUI _returnvalue (Variables|Default|GetPause%20Menu%20Widget) "DoNotLock" true false)
      (Variables|/Script/Engine.PlayerController|SetbShowMouseCursor (Game|GetPlayerController 0) true)
      (Game|SetGamePaused true)
      (else
        (Variables|Default|SetIsPauseMenuOpened%20? false)
        (Widget|RemovefromParent (Variables|Default|GetPause%20Menu%20Widget))
        (Game|SetGamePaused false)
        (Input|SetInputModeGameOnly _returnvalue false)
        (Variables|/Script/Engine.PlayerController|SetbShowMouseCursor (Game|GetPlayerController 0) false)))))

(fn ConstructionScript)